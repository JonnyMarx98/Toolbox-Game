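; DestructWall is a wall actor that shatters when another actor overlaps its Cube component.
; On a confirmed overlap it hides the Cube, disables its collision, spawns a batch of Break actors at random points within the wall's bounds, then destroys itself.
; An actor overlap that does not involve the Cube only prints a debug message.
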(event Collision|EventActorBeginOverlap
  (params (OtherActor :type Actor%20Object%20Reference))
  (bind (_origin _boxextent) (Collision|GetActorBounds false))
  (if (Collision|IsOverlappingActor (Variables|Default|GetCube) OtherActor :!class /Script/Engine.PrimitiveComponent)
    (Rendering|SetVisibility (Variables|Default|GetCube) false false)
    (Collision|SetCollisionEnabled (Variables|Default|GetCube) "NoCollision")
    (for _index (range 1 10)
      (Game|SpawnActorfromClass "/Game/Blueprints/Break.Break_C" (Math|Transform|MakeTransform (Math|Random|RandomPointinBoundingBox _origin _boxextent)) "AlwaysSpawn" 0 0))
    (Actor|DestroyActor)
    (else
      (Development|PrintString "No overlapping"))))

(fn ConstructionScript)